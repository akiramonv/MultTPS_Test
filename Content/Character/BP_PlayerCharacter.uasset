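; BP_PlayerCharacter is the player character Blueprint, handling walking, running, jumping, crouching and camera look from input events.
; Movement axes add input along the capsule's forward and right vectors, while look axes feed controller pitch and yaw.
; The forward/back axis event also sets max walk speed, switching from walk to run speed while the held run action keeps IsRun true.
; Jumping sets IsJump, which this graph never resets.
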(event `InputAction|RunForrest`
  (params (Key :type "Key Structure"))
  ;[1 1 1] Бег
  (:`Pressed`
    (set `self.isRun?` true))
  (:`Released`
    (set `self.isRun?` false)))

(event `InputAxis|MoveFB`
  (params (AxisValue :type "Float (single-precision)"))
  (bind _charactermovement (`self.CharacterMovement`))
  ;[1 1 1] Move
  (`self.AddMovementInput` (`SceneComponent.GetForwardVector` (`Character.CapsuleComponent` (`GameplayStatics.GetPlayerCharacter` 0))) AxisValue)
  (`|ExecutionSequence`
    (:`then_0`
      ;[1 1 1] Ходьба
      (set `CharacterMovementComponent.MaxWalkSpeed` 300.0 _charactermovement))
    (:`then_1`
      ;[1 1 1] Бег
      (if (`self.isRun?`)
        (set `CharacterMovementComponent.MaxWalkSpeed` 600.0 _charactermovement)))))

(event `InputAxis|MoveRL`
  (params (AxisValue :type "Float (single-precision)"))
  ;[1 1 1] Move
  (`self.AddMovementInput` (`SceneComponent.GetRightVector` (`Character.CapsuleComponent` (`GameplayStatics.GetPlayerCharacter` 0))) AxisValue))

(event `InputAxis|LookUD`
  (params (AxisValue :type "Float (single-precision)"))
  ;[1 1 1] Камера
  (`self.AddControllerPitchInput` AxisValue))

(event `InputAxis|LookRL`
  (params (AxisValue :type "Float (single-precision)"))
  ;[1 1 1] Камера
  (`self.AddControllerYawInput` AxisValue))

(event `InputAction|JumpUp`
  (params (Key :type "Key Structure"))
  ;[1 1 1] Прыжок
  (:`Pressed`
    (`self.Jump`)
    (set `self.isJump?` true)))

(event `InputAction|CrouchDown`
  (params (Key :type "Key Structure"))
  ;[1 1 1] Присед
  (:`Pressed`
    (`self.Crouch`))
  (:`Released`
    (`self.UnCrouch`)))

(fn `UserConstructionScript`)