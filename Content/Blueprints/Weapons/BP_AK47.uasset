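; AK-47 weapon Blueprint that the player can interact with to attach it to their character.
; Interact snaps the weapon to the skt_AK47 socket on player 0's character mesh, keeping relative scale, and always returns true.
; The event graph holds only disabled placeholder events, and the construction script just calls its parent.
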(fn `Interact`
  (returns (`isInterac?` :type Boolean))
  (`self.K2_AttachToComponent` (`Character.Mesh` (`GameplayStatics.GetPlayerCharacter` 0)) "skt_AK47" "SnapToTarget" "SnapToTarget" "KeepRelative")
  (return true))

(fn `UserConstructionScript`
  (`parent.UserConstructionScript`))